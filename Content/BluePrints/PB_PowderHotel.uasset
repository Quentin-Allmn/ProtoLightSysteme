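; PB_PowderHotel is an interactable, single-use powder source for the first-person player.
; On its Inetract event, it marks itself empty, casts player 0's character to BP_FirstPersonCharacter, adds AddPowder to NumberPowder and sets ColorofPowder to its own color.
; Later interactions only print an "Is Empty" message.
; The empty flag is set before the cast, so a failed cast still uses up the source.
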(event EventInetract
  (if (Variables|Default|GetIsEmpty)
    (Development|PrintString "Is Empty" true true "(R=0.846780,G=0.000000,B=1.000000,A=1.000000)")
    (else
      (Variables|Default|SetIsEmpty true)
      (bind _asbp_first_person_character (Utilities|Casting|CastToBP_FirstPersonCharacter (Game|GetPlayerCharacter 0)))
      (Variables|Default|SetAs%20BP%20First%20Person%20Character _asbp_first_person_character)
      (Variables|/Game/FirstPerson/Blueprints/BP_FirstPersonCharacter.BP_FirstPersonCharacter_C|SetNumberPowder _asbp_first_person_character (+ (Variables|/Game/FirstPerson/Blueprints/BP_FirstPersonCharacter.BP_FirstPersonCharacter_C|GetNumberPowder _asbp_first_person_character) (Variables|Default|GetAddPowder)))
      (Variables|/Game/FirstPerson/Blueprints/BP_FirstPersonCharacter.BP_FirstPersonCharacter_C|SetColorofPowder (Variables|Default|GetAs%20BP%20First%20Person%20Character) (Variables|Default|GetColorOfPowder)))))

(fn ConstructionScript)