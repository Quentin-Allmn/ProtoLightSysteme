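; BP_Candle_And_HidenText is an interactable candle that can reveal a hidden 3D text message.
; BeginPlay starts it unlit with the text set and hidden, and Inetract toggles the point light's intensity.
; UsePowder recolors the light and shows the text, without checking whether the candle is lit.
; Extinguishing through Inetract restores the base color and hides the text again.
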(event EventBeginPlay
  (bind _text3d (Variables|Default|GetText3D))
  (Rendering|Components|Light|SetIntensity (Variables|Default|GetPointLight) (Variables|Default|GetIntensity%20Null))
  (Class|Text3DComponent|SetText _text3d (Variables|Default|GetText))
  (Rendering|SetVisibility _text3d false false))

(event EventInetract
  (bind _pointlight (Variables|Default|GetPointLight))
  (if (Variables|Default|GetIsLighting)
    (Rendering|Components|Light|SetIntensity _pointlight (Variables|Default|GetIntensity%20Null))
    (Variables|Default|SetIsLighting (not (Variables|Default|GetIsLighting)))
    (Rendering|Components|Light|SetLightColor (Variables|Default|GetPointLight) (Variables|Default|GetBaseColor) true)
    (Rendering|SetVisibility (Variables|Default|GetText3D) false false)
    (else
      (Rendering|Components|Light|SetIntensity _pointlight (Variables|Default|GetIntensity))
      (Variables|Default|SetIsLighting true))))

(event EventUsePowder
  (Rendering|Components|Light|SetLightColor (Variables|Default|GetPointLight) (Variables|Default|GetPowder%20Color) true)
  (Rendering|SetVisibility (Variables|Default|GetText3D) true false))

(fn ConstructionScript)