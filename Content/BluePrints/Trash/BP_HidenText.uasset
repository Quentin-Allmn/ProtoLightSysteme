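; BP_HidenText is a hidden 3D text actor that is revealed when powder is used with a powdered candle.
; BeginPlay applies the configured text and hides it, while the box overlap stores whichever actor entered last as the candle reference.
; UsePowder casts that stored actor to BP_Candle and shows the text only if its IsPowder flag is set.
; Debug strings print on overlap and throughout the powder check.
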(event OnComponentBeginOverlap(Box)
  (params (OverlappedComponent :type Primitive%20Component%20Object%20Reference) (OtherActor :type Actor%20Object%20Reference) (OtherComp :type Primitive%20Component%20Object%20Reference) (OtherBodyIndex :type Integer) (bFromSweep :type Boolean) (SweepResult :type Hit%20Result%20Structure%20%28by%20ref%29))
  (bind _output_get (Variables|Default|SetCandleObject OtherActor))
  (Development|PrintString (Utilities|GetDisplayName _output_get)))

(event EventBeginPlay
  (bind _text3dcomponent (Variables|Default|GetText3DComponent))
  (Class|Text3DComponent|SetText _text3dcomponent (Variables|Default|Gettext))
  (Rendering|SetVisibility _text3dcomponent false false))

(event EventUsePowder
  (Development|PrintString "Use P")
  (bind _asbp_candle (Utilities|Casting|CastToBP_Candle (Variables|Default|GetCandleObject))
    (:then
      (if (Variables|/Game/BluePrints/BP_Candle.BP_Candle_C|GetIsPowder _asbp_candle)
        (Rendering|SetVisibility (Variables|Default|GetText3DComponent) true false)
        (Development|PrintString "Hello")
        (else
          (Development|PrintString "False"))))
    (:CastFailed
      (Development|PrintString "Cast Failed"))))

(fn ConstructionScript)